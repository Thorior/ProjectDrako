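; TestPlayer1_BP is a player character Blueprint that handles jumping and movement input, with a MovementDisabled flag gating movement and jump presses.
; Jump press and release drive Jump and StopJumping while tracking JumpPressed; release is never gated.
; Movement follows control-rotation yaw only, with MoveRight mapped to the forward vector and MoveUp to the right vector.
; MoveUp also stores its axis value in AxisValueToPass.
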(event EventBeginPlay)

(event Collision|EventActorBeginOverlap
  (params (OtherActor :type Actor%20Object%20Reference)))

(event EventTick
  (params (DeltaSeconds :type Float%20%28single-precision%29)))

(event Input|ActionEvents|InputActionJump
  (params (Key :type Key%20Structure :default "None"))
  ;[1 1 1] Jump System
  (:Pressed
    (if (not (Variables|Default|GetMovementDisabled))
      (Character|Jump)
      (Variables|Default|SetJumpPressed true)))
  (:Released
    (Variables|Default|SetJumpPressed false)
    (Character|StopJumping)))

(event Input|AxisEvents|InputAxisMoveRight
  (params (AxisValue :type Float%20%28single-precision%29))
  ;[1 1 1] Movement System
  (if (not (Variables|Default|GetMovementDisabled))
    (Pawn|Input|AddMovementInput (Math|Vector|GetForwardVector (Math|Rotator|MakeRotator 0.0 0.0 (.Yaw (Math|Rotator|BreakRotator (Pawn|GetControlRotation :!class /Script/Engine.Pawn))))) AxisValue false)))

(event Input|AxisEvents|InputAxisMoveUp
  (params (AxisValue :type Float%20%28single-precision%29))
  ;[1 1 1] Movement System
  (if (not (Variables|Default|GetMovementDisabled))
    (bind _output_get (Variables|Default|SetAxisValueToPass AxisValue))
    (Pawn|Input|AddMovementInput (Math|Vector|GetRightVector (Math|Rotator|MakeRotator 0.0 0.0 (.Yaw (Math|Rotator|BreakRotator (Pawn|GetControlRotation :!class /Script/Engine.Pawn))))) _output_get false)))

(fn ConstructionScript)