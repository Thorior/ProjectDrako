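; Chase camera actor that becomes the view target on begin play and follows PlayerToTrack at a Y offset.
; The construction script frames the player; each tick computes dead-zone X and Z values, Z being overridable by FixedZValue.
; The player's AxisValueToPass selects the movement branch: non-zero input replaces Z with a clamped height derived from the player and nudges clamped pitch, using input sampled within YMin/YMax.
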(event EventBeginPlay
  (Game|Player|SetViewTargetwithBlend (Game|GetPlayerController 0) self 0.0 "VTBlend_Linear" 0.0 false))

(event EventTick
  (params (DeltaSeconds :type Float%20%28single-precision%29))
  (bind _playertotrack (Variables|Default|GetPlayerToTrack))
  (bind _zoffset (Variables|Default|GetZOffset))
  (bind _playertotrack_2 (Variables|Default|GetPlayerToTrack))
  (bind _playertotrack_3 (Variables|Default|GetPlayerToTrack))
  (bind _returnvalue (Transformation|GetActorLocation _playertotrack_3))
  (bind _returnvalue_2 (Transformation|GetActorLocation _playertotrack))
  (bind _axisvaluetopass (Variables|/Game/Blueprints/TestPlayer1_BP.TestPlayer1_BP_C|GetAxisValueToPass _playertotrack_2))
  (bind _returnvalue_3 (+ (.z _returnvalue_2) _zoffset))
  (bind _newparam (CallFunction|GetNewXValue))
  (bind _output_get (Variables|Default|SetCameraX _newparam))
  (bind _newparam_2 (CallFunction|GetNewZValue))
  (Variables|Default|SetCameraZ _newparam_2)
  (if (== _axisvaluetopass 1.0)
    (bind _output_get_2 (Variables|Default|SetCameraZ (* (+ _returnvalue_3 (+ (Variables|/Game/Blueprints/TestPlayer1_BP.TestPlayer1_BP_C|GetAxisValueToPass _playertotrack) 1e+01)) 1.5)))
    (Transformation|SetActorLocation (Math|Vector|MakeVector (Variables|Default|GetCameraX) (+ (Variables|Default|GetYoffset) (.y _returnvalue_2)) (Math|Float|Clamp(Float) _output_get_2 _returnvalue_3 1.5e+03)) false false)
    (bind _newparam_3 (CallFunction|GetNewCameraRotation))
    (Transformation|SetActorRelativeRotation (Math|Rotator|MakeRotator 0.0 (Math|Float|ClampAngle (+ (* (* _newparam_3 -1.0) 0.25) (.pitch (Transformation|GetActorRotation self))) -35.0 0.0) -9e+01))
    (elif (== _axisvaluetopass 0.0)
      (Transformation|SetActorLocation (Math|Vector|MakeVector _output_get 0.0 0.0) false false)
      (else
        (bind _output_get_3 (Variables|Default|SetCameraZ (* 1.5 (+ (+ (.z _returnvalue) (Variables|Default|GetZOffset)) (+ (Variables|/Game/Blueprints/TestPlayer1_BP.TestPlayer1_BP_C|GetAxisValueToPass _playertotrack_3) -1e+01)))))
        (Transformation|SetActorLocation (Math|Vector|MakeVector 0.0 (+ (Variables|Default|GetYoffset) (.y _returnvalue)) (Math|Float|Clamp(Float) _output_get_3 (.z _returnvalue) 1.5e+03)) false false)
        (bind _newparam_4 (CallFunction|GetNewCameraRotation))
        (Transformation|SetActorRelativeRotation (Math|Rotator|MakeRotator 0.0 (Math|Float|ClampAngle (+ (* (* _newparam_4 -1.0) 0.25) (.pitch (Transformation|GetActorRotation self))) -35.0 -15.0) -9e+01))))))

(fn ConstructionScript
  (bind _playertotrack (Variables|Default|GetPlayerToTrack))
  (bind _returnvalue (Transformation|GetActorLocation _playertotrack))
  (Utilities|IsValid _playertotrack
    (:Is%20Valid
      (bind _output_get (Variables|Default|SetCameraX (.x _returnvalue)))
      (if (!= (Variables|Default|GetFixedZValue) 0.0)
        (Variables|Default|SetCameraZ (Variables|Default|GetFixedZValue))
        (else
          (bind _output_get_2 (Variables|Default|SetCameraZ (+ (.z _returnvalue) (Variables|Default|GetZdeadZone) (Variables|Default|GetZOffset))))))
      (Transformation|SetActorLocation (Math|Vector|MakeVector _output_get (+ (Variables|Default|GetYoffset) (.y _returnvalue)) _output_get_2) false false)
      (Transformation|SetActorRotation (Math|Rotator|MakeRotator 0.0 -15.0 (.yaw (Math|Rotator|FindLookatRotation (Transformation|GetActorLocation) (Transformation|GetActorLocation (Variables|Default|GetPlayerToTrack)))))))))

(fn GetNewXValue
  (bind _xdeadzone (Variables|Default|GetXDeadZone))
  (bind _xdeadzone_2 (Variables|Default|GetXDeadZone))
  (bind _playertotrack (Variables|Default|GetPlayerToTrack))
  (bind _playertotrack_2 (Variables|Default|GetPlayerToTrack))
  (bind _returnvalue (Transformation|GetActorLocation _playertotrack_2))
  (bind _returnvalue_2 (Transformation|GetActorLocation _playertotrack))
  (bind _returnvalue_3 (- (.x _returnvalue) _xdeadzone))
  (bind _returnvalue_4 (+ (.x _returnvalue_2) _xdeadzone_2))
  (if (> _returnvalue_3 (.x (Transformation|GetActorLocation)))
    (return _returnvalue_3)
    (elif (< _returnvalue_4 (.x (Transformation|GetActorLocation)))
      (return _returnvalue_4)
      (else
        (return (Variables|Default|GetCameraX))))))

(fn GetNewZValue
  (bind _playertotrack (Variables|Default|GetPlayerToTrack))
  (bind _playertotrack_2 (Variables|Default|GetPlayerToTrack))
  (bind _zdeadzone (Variables|Default|GetZdeadZone))
  (bind _zdeadzone_2 (Variables|Default|GetZdeadZone))
  (bind _returnvalue (Transformation|GetActorLocation _playertotrack_2))
  (bind _returnvalue_2 (Transformation|GetActorLocation _playertotrack))
  (bind _returnvalue_3 (- (.z _returnvalue) _zdeadzone))
  (bind _returnvalue_4 (+ (.z _returnvalue_2) _zdeadzone_2))
  (if (!= (Variables|Default|GetFixedZValue) 0.0)
    (return (Variables|Default|GetFixedZValue))
    (elif (> _returnvalue_3 (.z (Transformation|GetActorLocation)))
      (return _returnvalue_3)
      (elif (< _returnvalue_4 (.z (Transformation|GetActorLocation)))
        (return _returnvalue_4)
        (else
          (return (Variables|Default|GetCameraZ)))))))

(fn GetNewCameraRotation
  (bind _playertotrack (Variables|Default|GetPlayerToTrack))
  (bind _returnvalue (Transformation|GetActorLocation _playertotrack))
  (if (< (.y _returnvalue) (Variables|Default|GetYMax))
    (if (> (.y _returnvalue) (Variables|Default|GetYMin))
      (bind _output_get (Variables|Default|SetCameraPitch (Variables|/Game/Blueprints/TestPlayer1_BP.TestPlayer1_BP_C|GetAxisValueToPass (Variables|Default|GetPlayerToTrack))))
      (return _output_get))))